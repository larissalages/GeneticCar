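; SensorBP is a distance sensor actor in the Sedan folder that measures how close an obstacle lies ahead of it.
; SensorValue runs a Visibility line trace along the actor's forward vector over a fixed range.
; It turns hit distance into a normalized proximity, rising toward one as the obstacle nears and returning zero without a hit.
; The ShowLines flag draws the trace briefly for debugging.
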(fn `sensorValue`
  (returns (distance :type "Float (double-precision)"))
  (bind _returnvalue (`self.K2_GetActorLocation`))
  (bind (_outhit _returnvalue_2) (`KismetSystemLibrary.LineTraceSingle` :`Start` _returnvalue :`End` (+ _returnvalue (* (`self.GetActorForwardVector`) 1000)) :`TraceChannel` "TraceTypeQuery1" :`DrawDebugType` (select `bool` (`self.showLines`) :`true` "ForDuration" :!type "EDrawDebugTrace Enum") :`DrawTime` 0.15))
  (return (`KismetMathLibrary.SelectFloat` (- 1.0 (/ (`KismetMathLibrary.VSize` (- _returnvalue (`.Location` (`GameplayStatics.BreakHitResult` _outhit)))) 1000.0)) 0.0 _returnvalue_2)))

(fn `UserConstructionScript`)