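; Genetic algorithm manager Blueprint that builds the car population; the file holds only the spawning step, with no selection or evolution logic.
; The construction script clears Population, then adds SedanMLP child actor components on an NCarsX by NCarsY grid, storing each cast actor in the array.
; GetPos supplies each axis offset from index, count and spacing, apparently centering the grid on the actor.
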(fn ConstructionScript
  (Utilities|Array|Clear (Variables|Default|Getpopulation))
  (for _index (range 1 (Variables|Default|GetnCarsX))
    (LocalVariables|SetposX (Math|Conversions|ToFloat(Integer) (Utilities|GetPos _index (Variables|Default|GetnCarsX) (Variables|Default|GetdistX))))
    (for _index_2 (range 1 (Variables|Default|GetnCarsY))
      (LocalVariables|SetposY (Math|Conversions|ToFloat(Integer) (Utilities|GetPos _index_2 (Variables|Default|GetnCarsY) (Variables|Default|GetdistY))))
      (bind _returnvalue (AddComponent|AddChildActorComponent false (Math|Transform|MakeTransform (Math|Vector|MakeVector (LocalVariables|GetposX) (LocalVariables|GetposY) 0.0))))
      (ChildActorComponent|SetChildActorClass _returnvalue "/Game/Sedan/SedanMLP.SedanMLP_C")
      (bind _assedan_mlp (Utilities|Casting|CastToSedanMLP (Variables|/Script/Engine.ChildActorComponent|GetChildActor _returnvalue)))
      (Utilities|Array|Add (Variables|Default|Getpopulation) _assedan_mlp))))